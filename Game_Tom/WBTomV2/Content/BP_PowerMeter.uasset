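; BP_PowerMeter is an actor that shows an animated power meter and locks in a power value when the player presses.
; A timeline started on BeginPlay drives the widget component's fill and green-to-red colour, along with a text render showing power on a 0–100 scale.
; Tick polls HasPressed on the 2DSideScrollerCharacter, then stops the timeline, stores the meter value and sets PowerValueSet.
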(event `self.ReceiveBeginPlay`
  (bind _powerlevel_value (`self.PowerLevel Value`))
  (bind _aspower_meter (cast `/Game/PowerMeter` (`WidgetComponent.GetUserWidgetObject` (`self.Power_Meter`))))
  (set `self.PowerMeterReference` _aspower_meter)
  (bind (_direction _powermeteranimation) (`Timeline|PowerMeterAnimation`)
    (:`Update`
      (bind _returnvalue (`KismetMathLibrary.Lerp` 0.0 1.0 _powermeteranimation))
      (set `/Game/PowerMeter.PowerMeterValue` _returnvalue (`self.PowerMeterReference`))
      (bind _returnvalue_2 (`KismetMathLibrary.LinearColorLerp` (struct :`G` 1.0 :`B` 0.226251 :`A` 1.0) (struct :`R` 1.0 :`B` 0.008842 :`A` 1.0) _powermeteranimation))
      (set `/Game/PowerMeter.PowerMeterColour` _returnvalue_2 (`self.PowerMeterReference`))
      (`TextRenderComponent.K2_SetText` _powerlevel_value (`KismetTextLibrary.Conv_StringToText` (`KismetStringLibrary.Concat_StrStr` "Power" (`KismetStringLibrary.Conv_IntToString` (`KismetMathLibrary.Round` (* 100 _returnvalue))))))
      (`TextRenderComponent.SetTextRenderColor` _powerlevel_value (`KismetMathLibrary.Conv_LinearColorToColor` _returnvalue_2)))))

(event `self.ReceiveTick`
  (params (DeltaSeconds :type "Float (single-precision)"))
  ;[1 1 1] Comment
  (if (`/Game/2DSideScrollerBP/Blueprints/2DSideScrollerCharacter.hasPressed` (cast `/Game/2DSideScrollerBP/Blueprints/2DSideScrollerCharacter` (`GameplayStatics.GetPlayerPawn` 0) :!pure true))
    (`TimelineComponent.Stop` (`self.PowerMeterAnimation`))
    (set `self.PowerMeterValue ` (`/Game/PowerMeter.PowerMeterValue` (`self.PowerMeterReference`)))
    (set `self.bPower Value Set` true)))

(fn `UserConstructionScript`)